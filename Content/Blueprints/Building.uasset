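; Building actor that assembles a configurable building mesh with windows placed at its sockets in the Construction Script.
; When the Clear flag is set, it rebuilds a socket-to-window map with blacked-out tall-window defaults, then resets the flag.
; Each map entry adds a static mesh component at its socket, using that entry's mesh and material, with the second material slot chosen by window type.
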(event EventBeginPlay)

(event Collision|EventActorBeginOverlap
  (params (OtherActor :type Actor%20Object%20Reference)))

(event EventTick
  (params (DeltaSeconds :type Float%20%28single-precision%29)))

(fn ConstructionScript
  (bind _newvar_0 (Variables|Default|GetNewVar_0))
  (Components|StaticMesh|SetStaticMesh (Variables|Default|GetStaticMesh) (Variables|Default|GetNewVar_1))
  (Utilities|FlowControl|Sequence
    (:then_0
      (if (Variables|Default|Getclear)
        (Utilities|Map|Clear _newvar_0)
        (for _array_element (Transformation|GetAllSocketNames (Variables|Default|GetStaticMesh))
          (Development|PrintString (Utilities|String|ToString(Name) _array_element))
          (Utilities|Map|Add _newvar_0 _array_element (Utilities|Struct|MakeWindow "NewEnumerator1" 0 "/Game/Mesh/tallWindow.tallWindow")))
        (Variables|Default|Setclear false)))
    (:then_1
      (bind _keys (Utilities|Map|Keys (Variables|Default|GetNewVar_0)))
      (for _array_element_2 _keys
        (bind _returnvalue (AddComponent|AddStaticMeshComponent false (Transformation|GetSocketTransform (Variables|Default|GetStaticMesh) _array_element_2 "RTS_Actor")))
        (Components|StaticMesh|SetStaticMesh _returnvalue (.WindowMesh (Utilities|Struct|BreakWindow (.Value (Utilities|Map|Find (Variables|Default|GetNewVar_0) _array_element_2)))))
        (Rendering|Material|SetMaterial _returnvalue 0 (.Material (Utilities|Struct|BreakWindow (.Value (Utilities|Map|Find (Variables|Default|GetNewVar_0) _array_element_2)))))
        (Rendering|Material|SetMaterial _returnvalue 1 (Utilities|Select :Index (.WindowEnum (Utilities|Struct|BreakWindow (.Value (Utilities|Map|Find (Variables|Default|GetNewVar_0) _array_element_2)))) :NewEnumerator0 0 :NewEnumerator1 0 :NewEnumerator2 0))
        (Development|PrintString "Hello")))))