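; Door actor that toggles between open and closed when its SelectFoo event fires.
; Each call flips IsOpen, plays the matching one-shot open or close animation on the skeletal mesh, then calls the DoorOpen or DoorClose dispatcher.
; The construction script applies the Mesh variable to the skeletal mesh component.
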(event EventBeginPlay)

(event Collision|EventActorBeginOverlap
  (params (OtherActor :type Actor%20Object%20Reference)))

(event EventTick
  (params (DeltaSeconds :type Float%20%28single-precision%29)))

(event EventSelectFoo
  (params (NewParam :type Actor%20Component%20Object%20Reference))
  (bind _output_get (Variables|Default|SetbIsOpen (not (Variables|Default|GetbIsOpen))))
  (Components|Animation|PlayAnimation (Variables|Default|GetSkeletalMesh) (select _output_get "/Game/Mesh/doors/door_Anim_Armature_Open.door_Anim_Armature_Open" "/Game/Mesh/doors/door_Anim_Armature_close.door_Anim_Armature_close") false)
  (if (Variables|Default|GetbIsOpen)
    (Default|CallDoorOpen)
    (else
      (Default|CallDoorClose))))

(fn ConstructionScript
  (Class|SkinnedMeshComponent|SetSkeletalMesh (Variables|Default|GetSkeletalMesh) (Variables|Default|Getmesh) true))