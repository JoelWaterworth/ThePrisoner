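; Spline actor that tiles a static mesh along its spline as a chain of deforming spline mesh segments.
; The construction script divides the spline length by a segment-length variable, rounds down, and adds a SplineMeshComponent per segment.
; Each segment takes local-space start and end positions and tangents sampled by distance along the spline.
; It prints the last segment index for debugging; the event graph is empty.
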(event EventBeginPlay)

(event Collision|EventActorBeginOverlap
  (params (OtherActor :type Actor%20Object%20Reference)))

(event EventTick
  (params (DeltaSeconds :type Float%20%28single-precision%29)))

(fn ConstructionScript
  (bind _spline (Variables|Default|GetSpline))
  (bind _newvar_0 (Variables|Default|GetNewVar_0))
  (bind _spline_2 (Variables|Default|GetSpline))
  (bind _returnvalue (Spline|GetSplineLength _spline_2))
  (bind _returnvalue_2 (/ _returnvalue _newvar_0))
  (bind _returnvalue_3 (Math|Float|Floor _returnvalue_2))
  (bind _returnvalue_4 (- _returnvalue_3 1))
  (Development|PrintString (Utilities|String|ToString(Integer) _returnvalue_4))
  (for _index (range 0 _returnvalue_4)
    (bind _returnvalue_5 (AddComponent|AddSplineMeshComponent false))
    (bind _output_get (LocalVariables|SetNewLocalVar_0 _returnvalue_5))
    (Components|StaticMesh|SetStaticMesh _output_get (Variables|Default|GetNewVar_1))
    (SplineMesh|SetStartandEnd _returnvalue_5 (Spline|GetLocationatDistanceAlongSpline _spline (* _index _newvar_0) "Local") (Spline|GetTangentatDistanceAlongSpline _spline (* _index _newvar_0) "Local") (Spline|GetLocationatDistanceAlongSpline _spline (* (+ _index 1) _newvar_0) "Local") (Spline|GetTangentatDistanceAlongSpline _spline (* (+ _index 1) _newvar_0) "Local") true :!class /Script/Engine.SplineMeshComponent)))