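; CameraPan is a Behavior Tree task that sweeps a HeadCamera pawn back and forth between its starting and ending yaw angles.
; Each AI tick steps the positive-normalized yaw by TurnRate and delta time, signed by the IsPanningLeft blackboard bool.
; Overshooting the ending angle when panning left, or the starting angle otherwise, snaps to that limit and flips the bool.
; The task finishes successfully after each step.
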(event EventReceiveTickAI
  (params (OwnerController :type AI%20Controller%20Object%20Reference) (ControlledPawn :type Pawn%20Object%20Reference) (DeltaSeconds :type Float%20%28single-precision%29))
  (bind _ispanningleft (Variables|Default|GetIsPanningLeft))
  (bind _ispanningleft_2 (Variables|Default|GetIsPanningLeft))
  (bind _returnvalue (Class|BTFunctionLibrary|GetBlackboardValueasBool _ispanningleft))
  (bind _ashead_camera (Utilities|Casting|CastToHeadCamera ControlledPawn))
  (if (not (select _returnvalue (< (+ (Default|Makeroationpositive _ashead_camera (.Yaw (Math|Rotator|BreakRotator (Transformation|GetActorRotation _ashead_camera)))) (* DeltaSeconds (Variables|/Game/Blueprints/Camera/HeadCamera.HeadCamera_C|GetturnRate _ashead_camera) (select _returnvalue -1.0 1.0))) (Default|GetEndingAngle _ashead_camera)) (> (+ (Default|Makeroationpositive _ashead_camera (.Yaw (Math|Rotator|BreakRotator (Transformation|GetActorRotation _ashead_camera)))) (* DeltaSeconds (Variables|/Game/Blueprints/Camera/HeadCamera.HeadCamera_C|GetturnRate _ashead_camera) (select _returnvalue -1.0 1.0))) (Default|GetStartingAngle _ashead_camera))))
    (Transformation|SetActorRotation _ashead_camera (Math|Rotator|MakeRotator 0.0 0.0 (+ (Default|Makeroationpositive _ashead_camera (.Yaw (Math|Rotator|BreakRotator (Transformation|GetActorRotation _ashead_camera)))) (* DeltaSeconds (Variables|/Game/Blueprints/Camera/HeadCamera.HeadCamera_C|GetturnRate _ashead_camera) (select _returnvalue -1.0 1.0)))))
    (else
      (Transformation|SetActorRotation _ashead_camera (Math|Rotator|MakeRotator 0.0 0.0 (select _returnvalue (Default|GetEndingAngle _ashead_camera) (Default|GetStartingAngle _ashead_camera))))
      (Class|BTFunctionLibrary|SetBlackboardValueasBool _ispanningleft_2 (not (Class|BTFunctionLibrary|GetBlackboardValueasBool _ispanningleft_2)))))
  (AI|BehaviorTree|FinishExecute true))