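; CameraController is an AI controller for a security camera pawn (HeadCamera) that watches for the prisoner.
; It runs the BTCamera behavior tree on BeginPlay.
; On each perception update it reads the first actor's latest sensed stimulus, writes the CanSeePrisoner blackboard key, and tells the HeadCamera whether it sees or has lost the player.
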(event OnPerceptionUpdated(AIPerception)
  (params (UpdatedActors :type Array%20of%20Actor%20Object%20References))
  (bind _info (Class|AIPerceptionComponent|GetActorsPerception (Variables|Default|GetAIPerception) (Utilities|Array|Get(acopy) UpdatedActors)))
  (AI|Components|Blackboard|SetValueasBool (AI|GetBlackboard 0) (Utilities|Name|MakeLiteralName "CanSeePrisoner") (.bSuccessfullySensed (Utilities|Struct|BreakAIStimulus (Utilities|Array|Get(acopy) (.LastSensedStimuli (Utilities|Struct|BreakActorPerceptionBlueprintInfo _info))))))
  (bind _ashead_camera (Utilities|Casting|CastToHeadCamera (Pawn|GetControlledPawn)))
  (if (.bSuccessfullySensed (Utilities|Struct|BreakAIStimulus (Utilities|Array|Get(acopy) (.LastSensedStimuli (Utilities|Struct|BreakActorPerceptionBlueprintInfo _info)))))
    (Default|CanSeePlayer _ashead_camera)
    (else
      (Default|LostPlayer _ashead_camera))))

(event EventBeginPlay
  (AI|RunBehaviorTree "/Game/Blueprints/Camera/BTCamera.BTCamera"))

(fn ConstructionScript)