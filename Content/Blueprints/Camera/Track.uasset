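; Track is a behavior tree task that turns an AI-controlled HeadCamera pawn to face the player's pawn.
; On execute, it gets the HeadCamera from the owning CameraController and computes a look-at rotation from its CameraScene component to player 0's pawn.
; It applies only the yaw, zeroing pitch and roll, in one instant rotation, then finishes with success.
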(event EventReceiveExecute
  (params (OwnerActor :type Actor%20Object%20Reference))
  (bind _ascamera_controller (Utilities|Casting|CastToCameraController OwnerActor))
  (bind _ashead_camera (Utilities|Casting|CastToHeadCamera (Pawn|GetControlledPawn _ascamera_controller)))
  (Transformation|SetActorRotation _ashead_camera (Math|Rotator|MakeRotator 0.0 0.0 (.Yaw (Math|Rotator|BreakRotator (Math|Rotator|FindLookatRotation (Transformation|GetWorldLocation (Variables|/Game/Blueprints/Camera/HeadCamera.HeadCamera_C|GetCameraScene _ashead_camera)) (Transformation|GetActorLocation (Pawn|GetControlledPawn (Game|GetPlayerController 0))))))))
  (AI|BehaviorTree|FinishExecute true))