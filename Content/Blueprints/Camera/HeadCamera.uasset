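; HeadCamera is an AI-driven security camera that ends the game if its blackboard reports the prisoner visible when the bound Door opens.
; BeginPlay binds that door event, seeds the CameraController blackboard to pan left and switches its lights off.
; Player seen and lost events toggle the lights and print debug messages.
; The construction script orients two marker components and caches their world yaws as positive start and end angles, exposed through getters.
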(event Custom|DoorOpen
  (bind _ascamera_controller (Utilities|Casting|CastToCameraController (AI|GetAIController self)))
  (if (ScalableFloat|GetValueasBool (AI|GetBlackboard _ascamera_controller) (Utilities|Name|MakeLiteralName "CanSeePrisoner"))
    (bind _asbpgame_mode (Utilities|Casting|CastToBPGameMode (Game|GetGameMode)))
    (Default|GameOver _asbpgame_mode)))

(event Custom|Lost%20Player
  (for _array_element (Variables|Default|Getlights)
    (Rendering|Components|Light|SetIntensity (Variables|/Script/Engine.PointLight|GetPointLightComponent _array_element) 0.0))
  (Development|PrintString "Lost Player"))

(event Custom|Can%20see%20Player
  (for _array_element (Variables|Default|Getlights)
    (Rendering|Components|Light|SetIntensity (Variables|/Script/Engine.PointLight|GetPointLightComponent _array_element) 5e+03))
  (Development|PrintString "Can see Player"))

(event EventBeginPlay
  (Utilities|FlowControl|Sequence
    (:then_0
      (EventDispatchers|BindEventtoDoorOpen (Variables|Default|GetDoor) (delegate Custom|DoorOpen)))
    (:then_1
      (bind _ascamera_controller (Utilities|Casting|CastToCameraController (AI|GetAIController self)))
      (AI|Components|Blackboard|SetValueasBool (AI|GetBlackboard _ascamera_controller) (Utilities|Name|MakeLiteralName "IsPanningLeft") true))
    (:then_2
      (for _array_element (Variables|Default|Getlights)
        (Rendering|Components|Light|SetIntensity (Variables|/Script/Engine.Light|GetLightComponent _array_element) 0.0)))))

(fn ConstructionScript
  (Transformation|SetRelativeRotation (Variables|Default|Getfst) (Math|Rotator|MakeRotator 0.0 0.0 (Variables|Default|GetstartingAngle)) false false)
  (Transformation|SetRelativeRotation (Variables|Default|Getsnd) (Math|Rotator|MakeRotator 0.0 0.0 (Variables|Default|GetendingAngle)) false false)
  (Variables|Default|Setbaserotation (.yaw (Transformation|GetActorRotation)))
  (Variables|Default|Setsa (CallFunction|GetRotationOfComponent (Variables|Default|Getfst)))
  (Variables|Default|Setse (CallFunction|GetRotationOfComponent (Variables|Default|Getsnd))))

(fn NewFunction0)

(fn Makeroationpositive
  (params (NewParam :type Float%20%28single-precision%29))
  (bind _returnvalue (Math|Float|%(Float) NewParam 3.6e+02))
  (if (> _returnvalue 0.0)
    (return _returnvalue)
    (else
      (return (+ _returnvalue 3.6e+02)))))

(fn GetStartingAngle
  (return (Variables|Default|Getsa)))

(fn GetEndingAngle
  (return (Variables|Default|Getse)))

(fn GetRotationOfComponent
  (params (NewParam :type Scene%20Component%20Object%20Reference))
  (return (CallFunction|Makeroationpositive (.Yaw (Math|Rotator|BreakRotator (Transformation|GetWorldRotation NewParam))))))