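; ControlBoard is an actor Blueprint for a board built from a static mesh with instanced pieces placed at its sockets.
; The construction script adds one InstancedStaticMesh instance at each socket's world location and rotation, with scale fixed at one.
; At runtime, the SelectFoo_1 event calls Play on NewVar0 and ignores its parameter; the default BeginPlay, overlap and Tick events are disabled.
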(event Custom|SelectFoo_1
  (params (NewParam :type Actor%20Component%20Object%20Reference))
  (Default|Play (Variables|Default|GetNewVar_0)))

(event EventBeginPlay)

(event Collision|EventActorBeginOverlap
  (params (OtherActor :type Actor%20Object%20Reference)))

(event EventTick
  (params (DeltaSeconds :type Float%20%28single-precision%29)))

(fn ConstructionScript
  (bind _staticmesh (Variables|Default|GetStaticMesh))
  (for _array_element (Transformation|GetAllSocketNames _staticmesh)
    (Class|InstancedStaticMeshComponent|AddInstanceWorldSpace (Variables|Default|GetInstancedStaticMesh) (Math|Transform|MakeTransform (.Location (Math|Transform|BreakTransform (Transformation|GetSocketTransform _staticmesh _array_element "RTS_World"))) (.Rotation (Math|Transform|BreakTransform (Transformation|GetSocketTransform _staticmesh _array_element "RTS_World")))))))