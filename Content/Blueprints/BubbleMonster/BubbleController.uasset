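; BubbleController is the AI controller for the BubbleMonster enemy, linking its perception to a behavior tree.
; Start runs BubbleTree, and AttackAndStart also sets the AttackRegardless blackboard flag.
; Perception updates copy the first updated actor's first stimulus result into CanSeePrisoner and call EnemyFound on the controlled BubbleMonster when sensing succeeds.
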(event OnPerceptionUpdated(AIPerception)
  (params (UpdatedActors :type Array%20of%20Actor%20Object%20References))
  (bind _returnvalue (AI|GetBlackboard 0))
  (bind _info (Class|AIPerceptionComponent|GetActorsPerception (Variables|Default|GetAIPerception) (Utilities|Array|Get(acopy) UpdatedActors)))
  (Utilities|IsValid _returnvalue
    (:Is%20Valid
      (AI|Components|Blackboard|SetValueasBool _returnvalue (Utilities|Name|MakeLiteralName "CanSeePrisoner") (.bSuccessfullySensed (Utilities|Struct|BreakAIStimulus (Utilities|Array|Get(acopy) (.LastSensedStimuli (Utilities|Struct|BreakActorPerceptionBlueprintInfo _info))))))
      (bind _asbubble_monster (Utilities|Casting|CastToBubbleMonster (Pawn|GetControlledPawn)))
      (if (.bSuccessfullySensed (Utilities|Struct|BreakAIStimulus (Utilities|Array|Get(acopy) (.LastSensedStimuli (Utilities|Struct|BreakActorPerceptionBlueprintInfo _info)))))
        (Default|EnemyFound _asbubble_monster)))))

(event Custom|Start
  (bind _returnvalue (AI|RunBehaviorTree "/Game/Blueprints/BubbleMonster/BubbleTree.BubbleTree"))
  (if (not _returnvalue)
    (Development|PrintString "Didn't run")))

(event Custom|AttackAndStart
  (CallFunction|Start)
  (AI|Components|Blackboard|SetValueasBool (AI|GetBlackboard 0) (Utilities|Name|MakeLiteralName "AttackRegardless") true))

(fn ConstructionScript)