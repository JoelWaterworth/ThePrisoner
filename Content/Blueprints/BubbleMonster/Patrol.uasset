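; Behavior tree task that sends a BubbleController's pawn along numbered EnemyMarker actors as a patrol route.
; It searches all markers for the Blackboard NextMarker number and starts AIMoveTo, reporting success immediately while the move runs.
; Arrival increments the index; at the last marker it resets to zero and teleports the pawn just above that first marker instead of walking back.
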(event EventReceiveExecute
  (params (OwnerActor :type Actor%20Object%20Reference))
  (bind _nextmarker (Variables|Default|GetNextMarker))
  (bind _returnvalue (Class|BTFunctionLibrary|GetBlackboardValueasInt _nextmarker))
  (bind _returnvalue_2 (+ _returnvalue 1))
  (bind _asbubble_controller (Utilities|Casting|CastToBubbleController OwnerActor))
  (bind _array_element (CallFunction|Getmarker (Class|BTFunctionLibrary|GetBlackboardValueasInt (Variables|Default|GetNextMarker))))
  (Utilities|IsValid _array_element
    (:Is%20Valid
      (AI|AIMoveTo (Pawn|GetControlledPawn _asbubble_controller) "0, 0, 0" _array_element 5.0 false
        (:then
          (AI|BehaviorTree|FinishExecute true))
        (:OnSuccess
          (if (== _returnvalue_2 (Variables|Default|GetMarkerNumber))
            (Class|BTFunctionLibrary|SetBlackboardValueasInt (Variables|Default|GetNextMarker))
            (bind _array_element_2 (CallFunction|Getmarker (Class|BTFunctionLibrary|GetBlackboardValueasInt (Variables|Default|GetNextMarker))))
            (Transformation|SetActorLocation (Pawn|GetControlledPawn _asbubble_controller) (+ (Transformation|GetActorLocation _array_element_2) (Math|Vector|MakeVector 0.0 0.0 (+ (.z (.BoxExtent (Collision|GetActorBounds (Pawn|GetControlledPawn _asbubble_controller) false))) 1e+01))) false true)
            (AI|BehaviorTree|FinishExecute true)
            (else
              (Class|BTFunctionLibrary|SetBlackboardValueasInt (Variables|Default|GetNextMarker) _returnvalue_2))))
        (:OnFail
          (AI|BehaviorTree|FinishExecute false))))
    (:Is%20Not%20Valid
      (Development|PrintString "Marker invalid"))))

(fn Getmarker
  (params (B :type Integer))
  (bind _outactors (Actor|GetAllActorsOfClass "/Game/Blueprints/BubbleMonster/EnemyMarker.EnemyMarker_C"))
  (Variables|Default|SetMarkerNumber (Utilities|Array|Length _outactors))
  (bind _array_element (Utilities|Array|ForEachLoopwithBreak _outactors)
    (:LoopBody
      (if (== (Variables|/Game/Blueprints/BubbleMonster/EnemyMarker.EnemyMarker_C|GetMarkerNumber _array_element) B)
        (return _array_element)))
    (:Completed
      (return 0))))