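; First-person style player Blueprint that handles movement, mouse look, object selection and the game-over state.
; Axis inputs move the player along the camera's forward and right vectors and turn the controller's yaw and pitch.
; Select fires a visibility line trace from the camera, with persistent debug drawing, and calls SelectFooMessage on hit actors implementing SelectInterface.
; The GameOver event shows a message widget and disables input.
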(event Custom|GameOver
  (params (Message :type Text))
  (bind _returnvalue (Game|GetPlayerController 0))
  (bind _returnvalue_2 (UserInterface|CreateWidget "/Game/Blueprints/GameOver.GameOver_C" _returnvalue Message))
  (UserInterface|Viewport|AddtoViewport _returnvalue_2 0)
  (Input|DisableInput _returnvalue))

(event Input|ActionEvents|InputActionSelect
  (params (Key :type Key%20Structure))
  (bind _camera (Variables|Default|GetCamera))
  (bind _returnvalue (Transformation|GetWorldLocation _camera))
  (:Pressed
    (bind (_outhit _returnvalue_2) (Collision|LineTraceByChannel _returnvalue (+ _returnvalue (* (Math|Vector|GetForwardVector _camera) (Variables|Default|GetSelectDistance))) "TraceTypeQuery1" false 0 "Persistent"))
    (if _returnvalue_2
      (if (Utilities|DoesObjectImplementInterface (.HitActor (Collision|BreakHitResult _outhit)) "/Game/Blueprints/SelectInterface.SelectInterface_C")
        (Class|SelectInterface|SelectFoo(Message) (.HitActor (Collision|BreakHitResult _outhit)))))))

(event Input|AxisEvents|InputAxisMoveForward
  (params (AxisValue :type Float%20%28single-precision%29))
  ;[1 1 1] WASD movement
  (Pawn|Input|AddMovementInput (Math|Vector|GetForwardVector (Variables|Default|GetCamera)) AxisValue false))

(event Input|AxisEvents|InputAxisMoveRight
  (params (AxisValue :type Float%20%28single-precision%29))
  ;[1 1 1] WASD movement
  (Pawn|Input|AddMovementInput (Math|Vector|GetRightVector (Variables|Default|GetCamera)) AxisValue false))

(event Input|AxisEvents|InputAxisLookUp
  (params (AxisValue :type Float%20%28single-precision%29))
  ;[1 1 1] Mouse Controls
  (Pawn|Input|AddControllerPitchInput AxisValue))

(event Input|AxisEvents|InputAxisLookRight
  (params (AxisValue :type Float%20%28single-precision%29))
  ;[1 1 1] Mouse Controls
  (Pawn|Input|AddControllerYawInput AxisValue))

(fn ConstructionScript)