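; BPNote is a pickup actor for a note that the player collects by selecting it.
; The construction script applies a material variable to its static mesh.
; On SelectActor it casts the player pawn to Player, applies that same material to the player's mesh, sets HasNote to true, and destroys itself.
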(event EventBeginPlay)

(event Collision|EventActorBeginOverlap
  (params (OtherActor :type Actor%20Object%20Reference)))

(event EventSelectActor
  (params (NewParam :type Actor%20Component%20Object%20Reference))
  (bind _asplayer (Utilities|Casting|CastToPlayer (Game|Player|GetPlayerPawn 0)))
  (Rendering|Material|SetMaterial (Variables|/Game/Blueprints/Player.Player_C|GetStaticMesh _asplayer) 0 (Variables|Default|GetNewVar_0))
  (Variables|/Game/Blueprints/Player.Player_C|SetbHasNote _asplayer true)
  (Actor|DestroyActor))

(event EventTick
  (params (DeltaSeconds :type Float%20%28single-precision%29)))

(fn ConstructionScript
  (Rendering|Material|SetMaterial (Variables|Default|GetStaticMesh) 0 (Variables|Default|GetNewVar_0)))