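; BPGameMode is the game mode Blueprint that handles game over and level restart.
; GameOver waits a configurable delay, forwards the message to the player pawn, then after a second delay silences the audio of every BubbleMonster in the level.
; Restart reopens the NewMap level by name.
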(event Custom|Restart
  (Game|OpenLevel(byName) "NewMap"))

(event Custom|GameOver
  (params (Message :type Text))
  (Utilities|FlowControl|Delay (Variables|Default|GetGameOverDelay))
  (bind _asplayer (Utilities|Casting|CastToPlayer (Game|Player|GetPlayerPawn 0)))
  (Default|GameOver _asplayer Message)
  (Utilities|FlowControl|Delay (Variables|Default|GetSoundCutOffDelay))
  (bind _outactors (Actor|GetAllActorsOfClass "/Game/Blueprints/BubbleMonster/BubbleMonster.BubbleMonster_C"))
  (for _array_element _outactors
    (Audio|Components|Audio|SetVolumeMultiplier (Variables|/Game/Blueprints/BubbleMonster/BubbleMonster.BubbleMonster_C|GetAudio _array_element) 0.0 :!class /Script/Engine.AudioComponent)))

(event EventBeginPlay)

(event EventTick
  (params (DeltaSeconds :type Float%20%28single-precision%29)))

(fn ConstructionScript)